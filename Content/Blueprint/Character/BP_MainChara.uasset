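; Main player character Blueprint handling camera-relative movement, look, sprint and an acrobatic moveset of several jumps, a backflip and a roll slide.
; Short, medium and long jumps share a forward-launch function that also honors a coyote-time window opened when falling starts.
; Slide plays a roll montage in Flying mode with capsule collision disabled, then restores both.
; The construction script applies exposed movement and jump tuning variables.
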(event Custom|HorizontalMovement
  (params (ActionValueX :type Float%20%28double-precision%29))
  (bind _returnvalue (Pawn|GetControlRotation :!class /Script/Engine.Pawn))
  ;[1 1 1] Horizontal and Vertical Movement
  (Pawn|Input|AddMovementInput (Math|Vector|GetRightVector (Math|Rotator|MakeRotator (.roll _returnvalue) 0.0 (.yaw _returnvalue))) ActionValueX false))

(event Custom|VerticalMovement
  (params (ActionValueY :type Float%20%28double-precision%29))
  ;[1 1 1] Horizontal and Vertical Movement
  (Pawn|Input|AddMovementInput (Math|Vector|GetForwardVector (Math|Rotator|MakeRotator 0.0 0.0 (.yaw (Pawn|GetControlRotation :!class /Script/Engine.Pawn)))) ActionValueY false))

(event Custom|ShortJump
  (Utilities|CoyoteeandRegularJump (Variables|Mesh|Exposed|Jump|GetShortJumpLaunchVelocity) (Variables|Mesh|Exposed|Jump|GetShortJumpLaunchVelocityZ)))

(event Custom|LongJump
  (Utilities|CoyoteeandRegularJump (Variables|Mesh|Exposed|Jump|GetLongJumpLaunchVelocity) (Variables|Mesh|Exposed|Jump|GetLongJumpLaunchVelocityZ)))

(event Custom|MediumJump
  (Utilities|CoyoteeandRegularJump (Variables|Mesh|Exposed|Jump|GetMediumJumpLaunchVelocity) (Variables|Mesh|Exposed|Jump|GetMediumJumpLaunchVelocityZ)))

(event Custom|StopRunning
  ;[1 1 1] Running and stop running
  (Variables|/Script/Engine.CharacterMovementComponent|SetMaxWalkSpeed (Variables|Character|GetCharacterMovement) (Variables|Default|GetRegularWalkSpeed)))

(event Custom|CamRotationPitch
  (params (AxisValueY :type Float%20%28double-precision%29))
  ;[1 1 1] Camera Control PItch and Yaw
  (Pawn|Input|AddControllerPitchInput AxisValueY))

(event Custom|CamRotationYaw
  (params (AxisValueX :type Float%20%28double-precision%29))
  ;[1 1 1] Camera Control PItch and Yaw
  (Pawn|Input|AddControllerYawInput AxisValueX))

(event Custom|Run
  ;[1 1 1] Running and stop running
  (Utilities|FlowControl|Sequence
    (:then_0
      (Utilities|FlowControl|DoOnce false
        (:Completed
          (Variables|Default|SetRegularWalkSpeed (Variables|/Script/Engine.CharacterMovementComponent|GetMaxWalkSpeed (Variables|Character|GetCharacterMovement))))))
    (:then_1
      (Variables|/Script/Engine.CharacterMovementComponent|SetMaxWalkSpeed (Variables|Character|GetCharacterMovement) (Variables|Mesh|Exposed|GetSprintSpeed)))))

(event Custom|StopJump
  ;[1 1 1] Stop Jumping
  (Character|StopJumping))

(event Custom|RegularJump
  (Character|Jump))

(event Custom|BackflipJump
  (bind _capsulecomponent (Variables|Collision|GetCapsuleComponent))
  (bind _backflipjumpstrenght (Variables|Mesh|Exposed|BackflipJump|GetBackflipJumpStrenght))
  (bind _returnvalue (Math|Vector|GetForwardVector _capsulecomponent))
  (bind _returnvalue_2 (* _returnvalue _backflipjumpstrenght))
  ;[1 1 1] Backflip Jump
  (if (and (Variables|Default|GetCanUseBackflip) (Character|CanJump))
    (Variables|Default|SetCanUseBackflip false)
    (Character|LaunchCharacter (Math|Vector|MakeVector (.x _returnvalue_2) (.y _returnvalue_2) (Variables|Mesh|Exposed|BackflipJump|GetBackflipJumpVelocityZaxis)) false false)))

(event Custom|Slide
  ;[1 1 1] Sliding
  (Pawn|Components|CharacterMovement|SetMovementMode (Variables|Character|GetCharacterMovement) "MOVE_Flying" 0)
  (Collision|SetCollisionEnabled (Variables|Collision|GetCapsuleComponent) "NoCollision")
  (bind _returnvalue (Animation|PlayAnimMontage "/Game/Meshes/AMBP_Roll.AMBP_Roll" 1.0 "None"))
  (Utilities|FlowControl|Delay _returnvalue)
  (Collision|SetCollisionEnabled (Variables|Collision|GetCapsuleComponent) "QueryAndPhysics")
  (Pawn|Components|CharacterMovement|SetMovementMode (Variables|Character|GetCharacterMovement) "MOVE_Walking" 0))

(event EventOnMovementModeChanged
  (params (PrevMovementMode :type EMovementMode%20Enum :default "MOVE_None") (NewMovementMode :type EMovementMode%20Enum :default "MOVE_None") (PrevCustomMode :type Byte :default 0) (NewCustomMode :type Byte :default 0))
  ;[1 1 1] Coyote time
  (Utilities|FlowControl|Sequence
    (:then_0
      (if (and (Utilities|Enum|Equal(Enum) NewMovementMode "MOVE_Falling") (<= (.z (Variables|/Script/Engine.MovementComponent|GetVelocity (Variables|Character|GetCharacterMovement))) 0.0))
        (Variables|Default|SetCanUseCoyoteJump true)
        (Utilities|FlowControl|RetriggerableDelay (Variables|Default|GetTimeBeforeCoyoteJumpExpire))
        (Variables|Default|SetCanUseCoyoteJump false)))
    (:then_1
      (if (Character|CanJump)
        (Variables|Default|SetCanUseBackflip true)))))

(fn ConstructionScript
  (Utilities|FlowControl|Sequence
    (:then_0
      (Variables|/Script/Engine.CharacterMovementComponent|SetGravityScale (Variables|Character|GetCharacterMovement) (Variables|Mesh|Exposed|GetGravityScale)))
    (:then_1
      (Variables|Default|SetTimeBeforeCoyoteJumpExpire (Variables|Mesh|Exposed|GetCoyoteTimer)))
    (:then_2
      (Variables|/Script/Engine.CharacterMovementComponent|SetJumpZVelocity (Variables|Character|GetCharacterMovement) (Variables|Mesh|Exposed|GetRegularJumpVelocityZ)))
    (:then_3
      (Variables|Default|SetJumpMaxHoldTime (Variables|Mesh|Exposed|GetJump%20MaxHoldTime)))
    (:then_4
      (Variables|/Script/Engine.CharacterMovementComponent|SetAirControl (Variables|Character|GetCharacterMovement) (Variables|Mesh|Exposed|GetAir%20Control)))
    (:then_5
      (Variables|/Script/Engine.CharacterMovementComponent|SetRotationRate (Variables|Character|GetCharacterMovement) (Variables|Mesh|Exposed|GetCharacterRotationRate)))))