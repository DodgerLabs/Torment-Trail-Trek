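; BP_PC_LobbyController is the lobby player controller, handling lobby UI, ready status and character selection.
; It creates a host or client screen based on authority and forwards player-list updates to that widget.
; SetReadyStatus toggles the player's ready flag and has GM_Lobby refresh the list.
; ChangeCharacter respawns and possesses a new pawn in place, while SetCharacterClass saves the chosen mesh through SavePlayerAppearence.
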(event Custom|CreateMenus
  (Networking|SwitchHasAuthority
    (:Authority
      (bind _returnvalue (UserInterface|CreateWidget "/Game/OnlineMenuSystem/W_LobbyHostScreen.W_LobbyHostScreen_C"))
      (bind _output_get (Variables|Default|SetLobbyWidget _returnvalue))
      (UserInterface|Viewport|AddtoViewport _output_get 0))
    (:Remote
      (bind _returnvalue_2 (UserInterface|CreateWidget "/Game/OnlineMenuSystem/W_LobbyClientScreen.W_LobbyClientScreen_C"))
      (bind _output_get_2 (Variables|Default|SetLobbyWidget _returnvalue_2))
      (UserInterface|Viewport|AddtoViewport _output_get_2 0))))

(event Custom|UpdatePlayerList
  (params (PlayerInfo :type Array%20of%20Struct%20Player%20Info%20Structures))
  (Variables|Default|SetPlayer%20Info PlayerInfo)
  (Networking|SwitchHasAuthority
    (:Authority
      (bind _asw_lobby_host_screen (Utilities|Casting|CastToW_LobbyHostScreen (Variables|Default|GetLobbyWidget)))
      (Default|UpdatePLayerLIst _asw_lobby_host_screen (Variables|Default|GetPlayer%20Info)))
    (:Remote
      (bind _asw_lobby_client_screen (Utilities|Casting|CastToW_LobbyClientScreen (Variables|Default|GetLobbyWidget)))
      (Default|UpdatePlayerList _asw_lobby_client_screen (Variables|Default|GetPlayer%20Info)))))

(event Custom|ChangeCharacter
  (params (NewCharacter :type BP%20Third%20Person%20Character%20Class%20Reference))
  (bind _returnvalue (Pawn|GetControlledPawn))
  (Variables|Default|SetSpawnTransform (Transformation|GetActorTransform _returnvalue))
  (Actor|DestroyActor _returnvalue)
  (bind _returnvalue_2 (Game|SpawnActorfromClass NewCharacter (Variables|Default|GetSpawnTransform) "Undefined" "MultiplyWithRoot" 0 0))
  (Pawn|Possess _returnvalue_2))

(event Custom|SetCharacterClass
  (params (InputPin :type BP%20Third%20Person%20Character%20Class%20Reference))
  (bind _structout (Utilities|Struct|SetmembersinStruct_PlayerAppearence (Variables|Default|GetS_PlayerAppearence) InputPin))
  (CallFunction|SavePlayerAppearence _structout))

(event Custom|SetReadyStatus
  (bind _playerinfo (Variables|Default|GetPlayerInfo))
  (Utilities|Struct|SetmembersinStruct_PlayerInfo _playerinfo (not (Utilities|Struct|BreakStruct_PlayerInfo _playerinfo)))
  (bind _asgm_lobby (Utilities|Casting|CastToGM_Lobby (Game|GetGameMode)))
  (Default|UpdatePlayerList _asgm_lobby))

(event EventBeginPlay
  (bind _returnvalue (Game|GetPlayerController 0))
  (CallFunction|CreateMenus)
  ;[1 0 0] Comment
  (Variables|/Script/Engine.PlayerController|SetbShowMouseCursor _returnvalue false)
  (Input|SetInputModeGameOnly _returnvalue false))

(fn ConstructionScript)