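; Lobby game mode that tracks connected lobby player controllers and shares their player info list with each of them.
; On PostLogin it registers the controller and its info, labeling the local host as "Host" and always ready.
; UpdatePlayerList rebuilds the info list from all registered controllers, applying the same host override.
; Both events wait briefly before pushing the list to every controller's UpdatePlayerList.
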(event Custom|UpdatePlayerList
  (Utilities|Array|Clear (Variables|Default|GetConnectedPlayerInfo))
  (for _array_element (Variables|Default|GetConnectedPlayer)
    (if (Pawn|IsLocalPlayerController _array_element)
      (bind _output_get (Variables|/Game/Blueprint/BP_PC_LobbyController.BP_PC_LobbyController_C|SetPlayerInfo _array_element (Utilities|Struct|MakeStruct_PlayerInfo "Host" true)))
      (Utilities|Array|Add (Variables|Default|GetConnectedPlayerInfo) _output_get)
      (else
        (Utilities|Array|Add (Variables|Default|GetConnectedPlayerInfo) (Variables|/Game/Blueprint/BP_PC_LobbyController.BP_PC_LobbyController_C|GetPlayerInfo _array_element)))))
  (Utilities|FlowControl|Delay 0.2)
  (for _array_element_2 (Variables|Default|GetConnectedPlayer)
    (Default|UpdatePlayerList _array_element_2 (Variables|Default|GetConnectedPlayerInfo))))

(event EventPostLogin
  (params (NewPlayer :type Player%20Controller%20Object%20Reference))
  (bind _asbp_pc_lobby_controller (Utilities|Casting|CastToBP_PC_LobbyController NewPlayer))
  (Utilities|Array|Add (Variables|Default|GetConnectedPlayer) _asbp_pc_lobby_controller)
  (if (Pawn|IsLocalController _asbp_pc_lobby_controller)
    (bind _output_get (Variables|/Game/Blueprint/BP_PC_LobbyController.BP_PC_LobbyController_C|SetPlayerInfo _asbp_pc_lobby_controller (Utilities|Struct|MakeStruct_PlayerInfo "Host" true)))
    (Utilities|Array|Add (Variables|Default|GetConnectedPlayerInfo) _output_get)
    (else
      (Utilities|Array|Add (Variables|Default|GetConnectedPlayerInfo) (Variables|/Game/Blueprint/BP_PC_LobbyController.BP_PC_LobbyController_C|GetPlayerInfo _asbp_pc_lobby_controller))))
  (Utilities|FlowControl|Delay 0.2)
  (for _array_element (Variables|Default|GetConnectedPlayer)
    (Default|UpdatePlayerList _array_element (Variables|Default|GetConnectedPlayerInfo))))

(fn ConstructionScript)